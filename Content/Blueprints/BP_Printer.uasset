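; BP_Printer is a printer actor that prints report clues into the world.
; PrintClue plays the printer sound on every call, then checks the AlreadyPrint list for the given report ID.
; For a new ID it spawns a BP_I_Clue at the ClueSpawn transform, assigns the ID, enables blocking collision on its mesh, and records the ID so each report prints only once.
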(event `self.ReceiveBeginPlay`
  (`parent.ReceiveBeginPlay`))

(fn `PrintClue`
  (params (Id_rapport :type String))
  (`GameplayStatics.PlaySound2D` "/Game/Sounds/Printer/printer.printer" 1.0 1.0 0.0 null null)
  (for _array_element (`self.AlreadyPrint`)
    (set `self.Exists` (or (`self.Exists`) (`KismetStringLibrary.EqualEqual_StrStr` _array_element Id_rapport))))
  (if (not (`self.Exists`))
    (bind _returnvalue (`|SpawnActorFromClass` "/Game/Blueprints/Interractables/BP_I_Clue.BP_I_Clue_C" (`SceneComponent.K2_GetComponentToWorld` (`self.ClueSpawn`)) "Undefined" "MultiplyWithRoot" null null))
    (set `/Game/Blueprints/Interractables/BP_I_Clue.Id_rapport` Id_rapport _returnvalue)
    (`PrimitiveComponent.SetCollisionProfileName` (`/Game/Blueprints/Interractables/BP_Interractable.StaticMesh` _returnvalue) "BlockAllDynamic" true)
    (`KismetArrayLibrary.Array_AddUnique` (`self.AlreadyPrint`) Id_rapport)))

(fn `UserConstructionScript`
  (`parent.UserConstructionScript`))