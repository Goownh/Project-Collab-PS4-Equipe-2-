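; BP_Canvas is a paint canvas, apparently for an in-game PC, that the player draws on with the mouse and can print as a clue.
; BeginPlay and ResetCanvas build a fresh render target, plane material and brush material.
; Paint input traces under the cursor, converts the hit to UV and stamps the brush at grid-snapped positions.
; OpenCanvas/CloseCanvas toggle the plane; PrintCanvas spawns a BP_I_Clue at BP_Printer wearing the canvas material.
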(event `self.ReceiveBeginPlay`
  (`|ExecutionSequence` :!label _label
    (:`then_0`
      (bind _returnvalue (`KismetRenderingLibrary.CreateRenderTarget2D` 1024 1024))
      (bind _output_get (set `self.RenderTarget` _returnvalue))
      (`KismetRenderingLibrary.ClearRenderTarget2D` _output_get (struct :`R` 1.0 :`G` 1.0 :`B` 1.0 :`A` 1.0)))
    (:`then_1`
      (bind _returnvalue_2 (`KismetMaterialLibrary.CreateDynamicMaterialInstance` "/Game/Materials/M_PCPaintCanvas.M_PCPaintCanvas"))
      (`MaterialInstanceDynamic.SetTextureParameterValue` _returnvalue_2 "RenderTarget" (`self.RenderTarget`))
      (`PrimitiveComponent.SetMaterial` (`self.Plane`) 0 _returnvalue_2))
    (:`then_2`
      (bind _returnvalue_3 (`KismetMaterialLibrary.CreateDynamicMaterialInstance` "/Game/Materials/M_PcPaintBrush.M_PcPaintBrush"))
      (set `self.BrushMaterial` _returnvalue_3))))

(event `ResetCanvas`
  (goto _label))

(event `EnhancedInput|/Game/Input/Actions/IA_Paint`
  (params (ActionValue :type "Float (double-precision)") (ElapsedSeconds :type "Float (double-precision)") (TriggeredSeconds :type "Float (double-precision)") (InputAction :type "InputAction Object Reference" :default "/Game/Input/Actions/IA_Paint.IA_Paint"))
  (bind (_worldlocation _worlddirection) (`PlayerController.DeprojectMousePositionToWorld` (`/Game/Blueprints/BP_FL_shortcut.GetController`)))
  (:`Triggered`
    (if (== ActionValue 1.0)
      (bind _outhit (`KismetSystemLibrary.LineTraceSingle` :`Start` _worldlocation :`End` (+ _worldlocation (* _worlddirection 1500.0)) :`TraceChannel` "TraceTypeQuery1" :`bTraceComplex` true :`bIgnoreSelf` false))
      (bind _asbp_canvas (cast `/Game/Blueprints/BP_Canvas` (`.HitActor` (`GameplayStatics.BreakHitResult` _outhit))))
      (`self.DrawBrush` _asbp_canvas (`self.BrushTexture`) (`self.Brush Size`) (`GameplayStatics.FindCollisionUV` _outhit)))))

(event `SetMaterialCluePrint`
  (params (Clue :type "PrimitiveComponent Object Reference"))
  (`KismetSystemLibrary.Delay` 0.2)
  (`PrimitiveComponent.SetMaterial` Clue 0 (`PrimitiveComponent.GetMaterial` (`/Game/Blueprints/BP_Canvas.Plane` (`/Game/Blueprints/BP_FL_shortcut.GetCanvas`)) 0)))

(fn `CloseCanvas`
  (bind _plane (`self.Plane`))
  (`PrimitiveComponent.SetCollisionProfileName` _plane "NoCollision" true)
  (`SceneComponent.SetVisibility` _plane false false))

(fn `DrawBrush`
  (params (BrushTexture :type "Texture2D Object Reference") (BrushSize :type "Float (double-precision)") (DrawLocation :type "Vector2D Structure"))
  (bind _brushsize (`local.BrushSize`))
  (`|ExecutionSequence`
    (:`then_0`
      (`MaterialInstanceDynamic.SetTextureParameterValue` (`self.BrushMaterial`) "BrushTexture" BrushTexture))
    (:`then_1`
      (bind (_canvas _size _context) (`KismetRenderingLibrary.BeginDrawCanvasToRenderTarget` (`self.RenderTarget`)))
      (bind (_x _y) (`KismetMathLibrary.BreakVector2D` (- (* _size DrawLocation) (/ (`local.BrushSize`) 2.0))))
      (`Canvas.K2_DrawMaterial` _canvas (`self.BrushMaterial`) (`KismetMathLibrary.MakeVector2D` (`KismetMathLibrary.GridSnap_Float` _x 10.0) (`KismetMathLibrary.GridSnap_Float` _y 10.0)) (`KismetMathLibrary.MakeVector2D` _brushsize _brushsize) (0.0 0.0) (1.0 1.0) 0.0 (0.5 0.5))
      (`KismetRenderingLibrary.EndDrawCanvasToRenderTarget` _context))))

(fn `OpenCanvas`
  (bind _plane (`self.Plane`))
  (`PrimitiveComponent.SetCollisionProfileName` _plane "BlockAllDynamic" true)
  (`SceneComponent.SetVisibility` _plane true false))

(fn `PrintCanvas`
  (bind _returnvalue (`GameplayStatics.GetActorOfClass` "/Game/Blueprints/BP_Printer.BP_Printer_C"))
  (bind _returnvalue_2 (`|SpawnActorFromClass` "/Game/Blueprints/Interractables/BP_I_Clue.BP_I_Clue_C" (`SceneComponent.K2_GetComponentToWorld` (`/Game/Blueprints/BP_Printer.ClueSpawn` _returnvalue)) "Undefined" "MultiplyWithRoot" null null))
  (set `/Game/Blueprints/Interractables/BP_I_Clue.Id_rapport` "E00" _returnvalue_2)
  (bind _staticmesh (`/Game/Blueprints/Interractables/BP_Interractable.StaticMesh` _returnvalue_2))
  (`PrimitiveComponent.SetCollisionProfileName` _staticmesh "BlockAllDynamic" true)
  (`self.SetMaterialCluePrint` _staticmesh))

(fn `UserConstructionScript`)