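; Blueprint function library of shortcut getters for the first-person player and key interactable actors.
; GetController and GetCharacter cast player index 0's controller and character to the project's first-person classes.
; GetPc, GetBoard, GetDrawer and GetDoor each use GetActorOfClass to return a single BP_I_ actor of that type, so they assume one instance of each in the level.
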(fn `GetBoard`
  (returns (ReturnValue :type "/Game/Blueprints/Interractables/BP_I_Board Object Reference"))
  (bind _returnvalue (`GameplayStatics.GetActorOfClass` null "/Game/Blueprints/Interractables/BP_I_Board.BP_I_Board_C"))
  (return _returnvalue))

(fn `GetCharacter`
  (returns (`AsBP First Person Character` :type "/Game/FirstPerson/Blueprints/BP_FirstPersonCharacter Object Reference"))
  (bind _asbp_first_person_character (cast `/Game/FirstPerson/Blueprints/BP_FirstPersonCharacter` (`GameplayStatics.GetPlayerCharacter` null)))
  (return _asbp_first_person_character))

(fn `GetController`
  (returns (`AsBP First Person Player Controller` :type "/Game/FirstPerson/Blueprints/BP_FirstPersonPlayerController Object Reference"))
  (bind _asbp_first_person_player_controller (cast `/Game/FirstPerson/Blueprints/BP_FirstPersonPlayerController` (`GameplayStatics.GetPlayerController` null)))
  (return _asbp_first_person_player_controller))

(fn `GetDoor`
  (returns (ReturnValue :type "/Game/Blueprints/Interractables/BP_I_Door Object Reference"))
  (bind _returnvalue (`GameplayStatics.GetActorOfClass` null "/Game/Blueprints/Interractables/BP_I_Door.BP_I_Door_C"))
  (return _returnvalue))

(fn `GetDrawer`
  (returns (ReturnValue :type "/Game/Blueprints/Interractables/BP_I_Drawer Object Reference"))
  (bind _returnvalue (`GameplayStatics.GetActorOfClass` null "/Game/Blueprints/Interractables/BP_I_Drawer.BP_I_Drawer_C"))
  (return _returnvalue))

(fn `GetPc`
  (returns (ReturnValue :type "/Game/Blueprints/Interractables/BP_I_PC Object Reference"))
  (bind _returnvalue (`GameplayStatics.GetActorOfClass` null "/Game/Blueprints/Interractables/BP_I_PC.BP_I_PC_C"))
  (return _returnvalue))