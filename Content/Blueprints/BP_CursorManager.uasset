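; BP_CursorManager picks which custom widget the player's mouse cursor shows, based on the current interaction state.
; Every Tick it walks a priority chain of boolean flags: PC, grab, pin, stamp, remove cable, board, then a default fallback.
; The matching widget is set on the controller's Default cursor slot, which is then made current.
; The grab flag clears itself once applied, while the other flags are only read here.
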(event `self.ReceiveTick`
  (params (DeltaSeconds :type "Float (single-precision)"))
  (bind _asbp_first_person_player_controller (`/Game/Blueprints/BP_FL_shortcut.GetController`))
  (bind _asbp_first_person_player_controller_2 (`/Game/Blueprints/BP_FL_shortcut.GetController`))
  (if (`self.OnPC`)
    (`PlayerController.SetMouseCursorWidget` (`/Game/Blueprints/BP_FL_shortcut.GetController`) "Default" (`self.PCCursor`))
    (set `PlayerController.CurrentMouseCursor` "Default" (`/Game/Blueprints/BP_FL_shortcut.GetController`))
    (elif (`self.OnGrab`)
      (`PlayerController.SetMouseCursorWidget` (`/Game/Blueprints/BP_FL_shortcut.GetController`) "Default" (`self.GrabCursor`))
      (set `PlayerController.CurrentMouseCursor` "Default" (`/Game/Blueprints/BP_FL_shortcut.GetController`))
      (set `self.OnGrab` false)
      (elif (`self.OnPin`)
        (`PlayerController.SetMouseCursorWidget` _asbp_first_person_player_controller "Default" (`self.PinCursor`))
        (set `PlayerController.CurrentMouseCursor` "Default" _asbp_first_person_player_controller)
        (elif (`self.OnStamp`)
          (`PlayerController.SetMouseCursorWidget` _asbp_first_person_player_controller_2 "Default" (`self.StampCursor`))
          (set `PlayerController.CurrentMouseCursor` "Default" _asbp_first_person_player_controller_2)
          (elif (`self.OnRemoveCable`)
            (`PlayerController.SetMouseCursorWidget` (`/Game/Blueprints/BP_FL_shortcut.GetController`) "Default" (`self.RemoveCableCursor`))
            (set `PlayerController.CurrentMouseCursor` "Default" (`/Game/Blueprints/BP_FL_shortcut.GetController`))
            (elif (`self.OnBoard`)
              (`PlayerController.SetMouseCursorWidget` (`/Game/Blueprints/BP_FL_shortcut.GetController`) "Default" (`self.HandCursor`))
              (set `PlayerController.CurrentMouseCursor` "Default" (`/Game/Blueprints/BP_FL_shortcut.GetController`))
              (else
                (`PlayerController.SetMouseCursorWidget` (`/Game/Blueprints/BP_FL_shortcut.GetController`) "Default" (`self.DefaultCursor`))
                (set `PlayerController.CurrentMouseCursor` "Default" (`/Game/Blueprints/BP_FL_shortcut.GetController`))))))))))

(fn `UserConstructionScript`)