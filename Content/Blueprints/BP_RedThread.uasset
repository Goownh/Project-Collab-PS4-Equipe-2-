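; BP_RedThread is an actor that draws a red thread between a start and end point, with a pin mesh at each end.
; On BeginPlay it adds a cable component, shortened below the point distance to limit sag, with material tiling scaled to length.
; It then passes itself to the WBP_RemoveThread widget, hides that widget's button and places the widget component beside the start point.
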(event `self.ReceiveBeginPlay`
  (bind _returnvalue (`AddComponent|NODE_AddCableComponent-1` :`RelativeTransform` (`KismetMathLibrary.MakeTransform` (`self.StartPoint`))))
  (set `self.CableComp` _returnvalue)
  ; Tracer le fil et ajuster sa taille pour éviter qu'il ne pende de trop
  (set `CableComponent.EndLocation` (`self.EndPoint`) (`self.CableComp`))
  (set `CableComponent.CableLength` (* (`KismetMathLibrary.Vector_Distance` (`self.StartPoint`) (`self.EndPoint`)) 0.8) (`self.CableComp`))
  ; Définir le material du fil et son nombre de répétition
  (`PrimitiveComponent.SetMaterial` (`self.CableComp`) 0 "/Game/Materials/Board/M_Red_Thread.M_Red_Thread")
  (set `CableComponent.TileMaterial` (* (`CableComponent.CableLength` (`self.CableComp`)) 0.1) (`self.CableComp`))
  (set `CableComponent.CableWidth` 1.0 (`self.CableComp`))
  ; Fais apparaître les punaise au chaque dout du fil
  (bind _returnvalue_2 (`AddComponent|NODE_AddStaticMeshComponent-2` :`RelativeTransform` (`KismetMathLibrary.MakeTransform` (`self.StartPoint`))))
  (`StaticMeshComponent.SetStaticMesh` _returnvalue_2 "/Game/Mesh/Asset/Board/SM_Pin.SM_Pin")
  (bind _returnvalue_3 (`AddComponent|NODE_AddStaticMeshComponent-3` :`RelativeTransform` (`KismetMathLibrary.MakeTransform` (`self.EndPoint`))))
  (`StaticMeshComponent.SetStaticMesh` _returnvalue_3 "/Game/Mesh/Asset/Board/SM_Pin.SM_Pin")
  ; Cacher l'ui de suppression des fils et les placer correctement au-dessus du fil (point de départ du fil)
  (bind _aswbp_remove_thread (cast `/Game/UI/Widgets/Board/WBP_RemoveThread` (`WidgetComponent.GetWidget` (`self.WidgetRemove`))))
  (set `/Game/UI/Widgets/Board/WBP_RemoveThread.Cable` self _aswbp_remove_thread)
  (`Widget.SetVisibility` (`/Game/UI/Widgets/Board/WBP_RemoveThread.Button_46` _aswbp_remove_thread) "Hidden")
  (`SceneComponent.K2_SetRelativeLocation` (`self.WidgetRemove`) (+ (`self.StartPoint`) (0.0 -5.0 0.0)) false false))

(fn `UserConstructionScript`)