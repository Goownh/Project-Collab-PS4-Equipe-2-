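; BP_PauseMenu opens and closes the pause menu and manages the on-screen cursor widget.
; T or Escape shows WBP_PauseMenu with UI-only input and look locked, recording whether the controller's Interract flag was already set.
; Continue removes the menu and restores either game input or the prior interaction's locked UI state, switching to Game-and-UI input when the clicked actor is a BP_I_Board.
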(event `self.ReceiveBeginPlay`
  (bind _returnvalue (`|CreateWidget` "/Game/UI/Widgets/WBP_Cursor.WBP_Cursor_C" (`/Game/Blueprints/BP_FL_shortcut.GetController`)))
  (bind _output_get (set `self.Cursor` _returnvalue))
  (`UserWidget.AddToViewport` _output_get 0))

(event `Key|T`
  (params (Key :type "Key Structure"))
  (bind _asbp_first_person_player_controller (`/Game/Blueprints/BP_FL_shortcut.GetController`))
  (bind _asbp_first_person_player_controller_2 (`/Game/Blueprints/BP_FL_shortcut.GetController`))
  (:`Pressed`
    (`Controller.SetIgnoreLookInput` _asbp_first_person_player_controller_2 true :!label _label)
    (bind _returnvalue (`|CreateWidget` "/Game/UI/Widgets/Menus/WBP_PauseMenu.WBP_PauseMenu_C" _asbp_first_person_player_controller_2))
    (bind _output_get (set `self.Pause` _returnvalue))
    (`UserWidget.AddToViewport` _output_get 0)
    (`WidgetBlueprintLibrary.SetInputMode_UIOnlyEx` _asbp_first_person_player_controller_2 null)
    (set `PlayerController.bEnableClickEvents` true _asbp_first_person_player_controller)
    (set `PlayerController.bShowMouseCursor` true _asbp_first_person_player_controller)
    (if (`/Game/FirstPerson/Blueprints/BP_FirstPersonPlayerController.Interract` _asbp_first_person_player_controller)
      (set `self.InInterractable` true)
      (`Widget.RemoveFromParent` (`self.Cursor`))
      (else
        (set `/Game/FirstPerson/Blueprints/BP_FirstPersonPlayerController.Interract` true _asbp_first_person_player_controller)))))

(event `Key|Escape`
  (params (Key :type "Key Structure"))
  (:`Pressed`
    (goto _label)))

(event `Continue`
  (bind _asbp_first_person_player_controller (`/Game/Blueprints/BP_FL_shortcut.GetController`))
  (bind _asbp_first_person_player_controller_2 (`/Game/Blueprints/BP_FL_shortcut.GetController`))
  (bind _returnvalue (`|CreateWidget` "/Game/UI/Widgets/WBP_Cursor.WBP_Cursor_C" (`/Game/Blueprints/BP_FL_shortcut.GetController`)))
  (bind _output_get (set `self.Cursor` _returnvalue))
  (`UserWidget.AddToViewport` _output_get 0)
  (`Controller.ResetIgnoreLookInput` _asbp_first_person_player_controller_2)
  (`Widget.RemoveFromParent` (`self.Pause`))
  (`WidgetBlueprintLibrary.SetInputMode_GameOnly` _asbp_first_person_player_controller_2)
  (set `PlayerController.bEnableClickEvents` true _asbp_first_person_player_controller)
  (if (`self.InInterractable`)
    (`Controller.SetIgnoreLookInput` _asbp_first_person_player_controller true)
    (`WidgetBlueprintLibrary.SetInputMode_UIOnlyEx` _asbp_first_person_player_controller null)
    (else
      (set `PlayerController.bShowMouseCursor` false _asbp_first_person_player_controller)
      (set `/Game/FirstPerson/Blueprints/BP_FirstPersonPlayerController.Interract` false _asbp_first_person_player_controller)))
  (set `self.InInterractable` false)
  (if (== (`GameplayStatics.GetObjectClass` (`/Game/FirstPerson/Blueprints/BP_FirstPersonPlayerController.ActorClick` _asbp_first_person_player_controller)) "/Game/Blueprints/Interractables/BP_I_Board.BP_I_Board_C")
    (`WidgetBlueprintLibrary.SetInputMode_GameAndUIEx` _asbp_first_person_player_controller null)))

(fn `UserConstructionScript`)