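; BP_Interractable_Child is an interactable actor variant that reveals a return arrow in a vote UI when interacted with.
; Its Interraction event calls SetUI, which casts the Widget component's widget to WBP_Vote and makes its WBPArrowReturn element visible.
; The construction script only calls the parent, and the BeginPlay, overlap and Tick events are unused placeholders.
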(event `self.Interraction`
  (`self.SetUI`))

(fn `SetUI`
  (bind _aswbp_vote (cast `/Game/UI/Widgets/VillagerPicture/WBP_Vote` (`WidgetComponent.GetWidget` (`self.Widget`))))
  (`Widget.SetVisibility` (`/Game/UI/Widgets/VillagerPicture/WBP_Vote.WBP_ArrowReturn` _aswbp_vote) "Visible"))

(fn `UserConstructionScript`
  (`parent.UserConstructionScript`))