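; Interactable villager picture for the board, with a vote widget bound to its character and the villager's material applied to a mesh that starts hidden.
; Zooming lerps the mesh by timeline from its original transform to the board's ClueExample transform while ignoring look input.
; Return reverses the lerp and makes the board the clicked actor again.
; Helper functions toggle the vote widget's UI collision and swap return arrows between picture and board.
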(event `self.ReceiveBeginPlay`
  (`parent.ReceiveBeginPlay`)
  (`SceneComponent.SetVisibility` (`self.StaticMesh`) false true)
  ; Récupère son identité pour se différencier
  (bind _aswbp_vote (cast `/Game/UI/Widgets/VillagerPicture/WBP_Vote` (`WidgetComponent.GetWidget` (`self.WidgetVote`))))
  (`/Game/UI/Widgets/VillagerPicture/WBP_Vote.setChara` _aswbp_vote (`self.charaSetted`) self)
  (`PrimitiveComponent.SetMaterial` (`self.StaticMesh`) 0 (`self.MaterialVillager`)))

(event `ZoomOnBoard`
  ; Zoom sur l'objet selon la caméra du tableau
  (bind _outactors (`GameplayStatics.GetAllActorsOfClass` "/Game/Blueprints/Interractables/BP_I_Board.BP_I_Board_C"))
  (for _array_element _outactors
    (bind _asbp_i_board (cast `/Game/Blueprints/Interractables/BP_I_Board` _array_element))
    (`Controller.SetIgnoreLookInput` (`GameplayStatics.GetPlayerController` 0) true)
    (bind (_direction _newtrack_0) (`Timeline|Timeline_1` :!via `PlayFromStart`)
      (:`Update`
        (bind (_returnvalue_location _returnvalue_rotation) (`KismetMathLibrary.BreakTransform` (`SceneComponent.K2_GetComponentToWorld` (`/Game/Blueprints/Interractables/BP_I_Board.ClueExample` _asbp_i_board))))
        (`SceneComponent.K2_SetWorldTransform` (`self.StaticMesh`) (`KismetMathLibrary.MakeTransform` (`KismetMathLibrary.VLerp` (`self.OriginalLocation`) _returnvalue_location _newtrack_0) (`KismetMathLibrary.RLerp` (`self.OriginalRotation`) _returnvalue_rotation _newtrack_0) (`self.originalScale`)) false false)))))

(event `DezoomBoard`
  ; Dézoom selon la caméra du tableau
  (`Controller.ResetIgnoreLookInput` (`GameplayStatics.GetPlayerController` 0))
  (bind _outactors (`GameplayStatics.GetAllActorsOfClass` "/Game/Blueprints/Interractables/BP_I_Board.BP_I_Board_C"))
  (for _array_element _outactors
    (bind _asbp_i_board (cast `/Game/Blueprints/Interractables/BP_I_Board` _array_element))
    (bind (_direction _newtrack_0) (`Timeline|Timeline_2` :!via `PlayFromStart`)
      (:`Update`
        (bind (_returnvalue_location _returnvalue_rotation) (`KismetMathLibrary.BreakTransform` (`SceneComponent.K2_GetComponentToWorld` (`/Game/Blueprints/Interractables/BP_I_Board.ClueExample` _asbp_i_board))))
        (`SceneComponent.K2_SetWorldTransform` (`self.StaticMesh`) (`KismetMathLibrary.MakeTransform` (`KismetMathLibrary.VLerp` _returnvalue_location (`self.OriginalLocation`) _newtrack_0) (`KismetMathLibrary.RLerp` _returnvalue_rotation (`self.OriginalRotation`) _newtrack_0) (`self.originalScale`)) false false)))))

(fn `CameraChange`
  (`self.ZoomOnBoard`)
  (`PrimitiveComponent.SetCollisionProfileName` (`self.WidgetVote`) "UI" true))

(fn `CheckDay`)

(fn `DisableUI`
  (`PrimitiveComponent.SetCollisionProfileName` (`self.WidgetVote`) "NoCollision" true)
  (bind _aswbp_vote (cast `/Game/UI/Widgets/VillagerPicture/WBP_Vote` (`WidgetComponent.GetWidget` (`self.WidgetVote`))))
  (`Widget.SetVisibility` (`/Game/UI/Widgets/VillagerPicture/WBP_Vote.WBP_ArrowReturn` _aswbp_vote) "Hidden"))

(fn `Return`
  (`self.DezoomBoard`)
  (set `/Game/FirstPerson/Blueprints/BP_FirstPersonPlayerController.ActorClick` (`/Game/Blueprints/BP_FL_shortcut.GetBoard`) (`/Game/Blueprints/BP_FL_shortcut.GetController`))
  (`self.DisableUI`)
  (bind _aswbp_arrow_return (cast `/Game/UI/Widgets/clue/WBP_ArrowReturn` (`WidgetComponent.GetWidget` (`/Game/Blueprints/Interractables/BP_I_Board.WidgetReturn` (`/Game/Blueprints/BP_FL_shortcut.GetBoard`)))))
  (`Widget.SetVisibility` _aswbp_arrow_return "Visible"))

(fn `SetUI`
  (bind _aswbp_vote (cast `/Game/UI/Widgets/VillagerPicture/WBP_Vote` (`WidgetComponent.GetWidget` (`self.WidgetVote`))))
  (`Widget.SetVisibility` (`/Game/UI/Widgets/VillagerPicture/WBP_Vote.WBP_ArrowReturn` _aswbp_vote) "Visible")
  (bind _aswbp_arrow_return (cast `/Game/UI/Widgets/clue/WBP_ArrowReturn` (`WidgetComponent.GetWidget` (`/Game/Blueprints/Interractables/BP_I_Board.WidgetReturn` (`/Game/Blueprints/BP_FL_shortcut.GetBoard`)))))
  (`Widget.SetVisibility` _aswbp_arrow_return "Hidden"))

(fn `UserConstructionScript`
  (`parent.UserConstructionScript`))