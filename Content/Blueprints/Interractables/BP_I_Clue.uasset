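; Interactable clue that the player inspects and files on the board or in the drawer, with material and widget content set from IdRapport and DT_Clue.
; InBoard, InDrawer and InLetter flags determine which WBP_Clue arrows appear and how storing or returning behaves.
; Board storage teleports the actor to the board's spawn point, while drawer storage records the ID and destroys the actor.
; On the board, timelines lerp the mesh to and from a close-up transform.
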(event `self.ReceiveBeginPlay`
  (bind _id_rapport (`self.Id_rapport`))
  (`parent.ReceiveBeginPlay`)
  (set `self.UsableForTuto` true)
  (`KismetSystemLibrary.Delay` 0.1)
  (bind _aswbp_clue (cast `/Game/UI/Widgets/clue/WBP_Clue` (`WidgetComponent.GetWidget` (`self.Widget`))))
  (`/Game/UI/Widgets/clue/WBP_Clue.SetClue` _aswbp_clue _id_rapport)
  (bind _returnvalue (`|GetDataTableRow` "/Game/Blueprints/Structures/DT_Clue.DT_Clue" (`KismetStringLibrary.Conv_StringToName` _id_rapport))
    (:`then`
      (`PrimitiveComponent.SetMaterial` (`self.StaticMesh`) 0 (`.MaterialClue_13_4B290FF24072822111A76C9F8A2E689F` (break `/Game/Blueprints/Structures/F_Clue` _returnvalue))))))

(event `self.Interraction`
  (if (`self.InBoard`)
    (`self.OnBoard`)
    (else
      (`self.SimpleClue`)
      (if (`/Game/Blueprints/BP_FL_shortcut.GetIsTuto`)
        (`KismetSystemLibrary.PrintText` "VA \"Je devrait le mettre sur le tableau pour le mettre en valeur.\"" true true (struct :`R` 1.0 :`A` 1.0) 10.0)))))

(event `StoreBoard`
  (bind _returnvalue (`/Game/Blueprints/BP_FL_shortcut.GetDrawer`))
  ; Ranger les indices où l'on souhaite
  (if (`self.InDrawer`)
    (`KismetArrayLibrary.Array_RemoveItem` (`/Game/Blueprints/Interractables/BP_I_Drawer.ListClue` _returnvalue) (`self.Id_rapport`))
    (`self.Interraction` _returnvalue)
    (set `self.InDrawer` false)
    (set `/Game/FirstPerson/Blueprints/BP_FirstPersonPlayerController.ActorClick` _returnvalue (`/Game/Blueprints/BP_FL_shortcut.GetController`))
    (`self.TeleportToBoard`)
    (elif (`self.InLetter`)
      (bind _outactors (`GameplayStatics.GetAllActorsOfClass` "/Game/Blueprints/Interractables/BP_I_letter.BP_I_letter_C"))
      (for _array_element _outactors
        (`self.Interraction` _array_element)
        (`self.TeleportToBoard`)
        (set `self.InLetter` false))
      (else
        (`self.Return`)
        (`self.TeleportToBoard`)))))

(event `StoreDrawer`
  ; Ranger les indices où l'on souhaite
  (if (`self.InLetter`)
    (`self.AddToDrawer`)
    (bind _outactors (`GameplayStatics.GetAllActorsOfClass` "/Game/Blueprints/Interractables/BP_I_letter.BP_I_letter_C"))
    (for _array_element _outactors
      (`self.Interraction` _array_element)
      (`self.K2_DestroyActor`))
    (elif (`self.InBoard`)
      (`self.Return`)
      (`self.AddToDrawer`)
      (set `/Game/FirstPerson/Blueprints/BP_FirstPersonPlayerController.ActorClick` (`/Game/Blueprints/BP_FL_shortcut.GetBoard`) (`/Game/Blueprints/BP_FL_shortcut.GetController`))
      (`self.K2_DestroyActor`)
      (else
        (`self.Return`)
        (`self.AddToDrawer`)
        (`self.K2_DestroyActor`)))))

(event `Letter`
  ; Affichage
  (bind _aswbp_clue (cast `/Game/UI/Widgets/clue/WBP_Clue` (`WidgetComponent.GetWidget` (`self.Widget`))))
  (`/Game/UI/Widgets/clue/WBP_Clue.ShowArrowBoard` _aswbp_clue)
  (`/Game/UI/Widgets/clue/WBP_Clue.ShowArrowDrawer` _aswbp_clue)
  (`/Game/UI/Widgets/clue/WBP_Clue.ShowVillagerImage` _aswbp_clue)
  (`PrimitiveComponent.SetCollisionProfileName` (`self.Widget`) "UI" true)
  (`self.SetControllerVariable`)
  (set `self.InLetter` true))

(event `DrawerOpen`
  ; Affichage
  (bind _aswbp_clue (cast `/Game/UI/Widgets/clue/WBP_Clue` (`WidgetComponent.GetWidget` (`self.Widget`))))
  (`/Game/UI/Widgets/clue/WBP_Clue.ShowArrowBoard` _aswbp_clue)
  (`/Game/UI/Widgets/clue/WBP_Clue.ShowArrowReturn` _aswbp_clue)
  (`/Game/UI/Widgets/clue/WBP_Clue.ShowVillagerImage` _aswbp_clue)
  (`PrimitiveComponent.SetCollisionProfileName` (`self.Widget`) "UI" true)
  (`self.SetControllerVariable`))

(event `OnBoard`
  ; Affichage
  (bind _aswbp_clue (cast `/Game/UI/Widgets/clue/WBP_Clue` (`WidgetComponent.GetWidget` (`self.Widget`))))
  (`/Game/UI/Widgets/clue/WBP_Clue.ShowArrowDrawer` _aswbp_clue)
  (`/Game/UI/Widgets/clue/WBP_Clue.ShowArrowReturn` _aswbp_clue)
  (`/Game/UI/Widgets/clue/WBP_Clue.ShowVillagerImage` _aswbp_clue)
  (`PrimitiveComponent.SetCollisionProfileName` (`self.Widget`) "UI" true)
  (`self.SetControllerVariable`)
  (bind _aswbp_arrow_return (cast `/Game/UI/Widgets/clue/WBP_ArrowReturn` (`WidgetComponent.GetWidget` (`/Game/Blueprints/Interractables/BP_I_Board.WidgetReturn` (`/Game/Blueprints/BP_FL_shortcut.GetBoard`)))))
  (`Widget.SetVisibility` _aswbp_arrow_return "Hidden"))

(event `SimpleClue`
  ; Affichage
  (bind _aswbp_clue (cast `/Game/UI/Widgets/clue/WBP_Clue` (`WidgetComponent.GetWidget` (`self.Widget`))))
  (`/Game/UI/Widgets/clue/WBP_Clue.ShowArrowBoard` _aswbp_clue)
  (`/Game/UI/Widgets/clue/WBP_Clue.ShowArrowDrawer` _aswbp_clue)
  (`/Game/UI/Widgets/clue/WBP_Clue.ShowArrowReturn` _aswbp_clue)
  (`/Game/UI/Widgets/clue/WBP_Clue.ShowVillagerImage` _aswbp_clue)
  (`PrimitiveComponent.SetCollisionProfileName` (`self.Widget`) "UI" true)
  (`self.SetControllerVariable`))

(event `ZoomOnBoard`
  (bind (_returnvalue_location _returnvalue_rotation) (`KismetMathLibrary.BreakTransform` (`SceneComponent.K2_GetComponentToWorld` (`/Game/Blueprints/Interractables/BP_I_Board.ClueExample` (`/Game/Blueprints/BP_FL_shortcut.GetBoard`)))))
  (`Controller.SetIgnoreLookInput` (`GameplayStatics.GetPlayerController` 0) true)
  (bind (_direction _newtrack_0) (`Timeline|Timeline_1` :!via `PlayFromStart`)
    (:`Update`
      (`SceneComponent.K2_SetWorldTransform` (`self.StaticMesh`) (`KismetMathLibrary.MakeTransform` (`KismetMathLibrary.VLerp` (`self.OriginalLocation`) _returnvalue_location _newtrack_0) (`KismetMathLibrary.RLerp` (`self.OriginalRotation`) _returnvalue_rotation _newtrack_0) (`self.originalScale`)) false false))))

(event `DezoomBoard`
  (bind (_returnvalue_location _returnvalue_rotation) (`KismetMathLibrary.BreakTransform` (`SceneComponent.K2_GetComponentToWorld` (`/Game/Blueprints/Interractables/BP_I_Board.ClueExample` (`/Game/Blueprints/BP_FL_shortcut.GetBoard`)))))
  (`Controller.ResetIgnoreLookInput` (`GameplayStatics.GetPlayerController` 0))
  (bind (_direction _newtrack_0) (`Timeline|Timeline_2` :!via `PlayFromStart`)
    (:`Update`
      (`SceneComponent.K2_SetWorldTransform` (`self.StaticMesh`) (`KismetMathLibrary.MakeTransform` (`KismetMathLibrary.VLerp` _returnvalue_location (`self.OriginalLocation`) _newtrack_0) (`KismetMathLibrary.RLerp` _returnvalue_rotation (`self.OriginalRotation`) _newtrack_0) (`self.originalScale`)) false false))))

(fn `AddToDrawer`
  (`KismetArrayLibrary.Array_Add` (`/Game/Blueprints/Interractables/BP_I_Drawer.ListClue` (`/Game/Blueprints/BP_FL_shortcut.GetDrawer`)) (`self.Id_rapport`))
  (set `self.InDrawer` true))

(fn `CameraChange`
  (if (`self.InBoard`)
    (`self.ZoomOnBoard`)
    (else
      (`self.ObjectZoom`)))
  (`PrimitiveComponent.SetCollisionProfileName` (`self.Widget`) "UI" true))

(fn `DisableUI`
  (`PrimitiveComponent.SetCollisionProfileName` (`self.Widget`) "NoCollision" true)
  (bind _aswbp_clue (cast `/Game/UI/Widgets/clue/WBP_Clue` (`WidgetComponent.GetWidget` (`self.Widget`))))
  (`/Game/UI/Widgets/clue/WBP_Clue.HideArrowBoard` _aswbp_clue)
  (`/Game/UI/Widgets/clue/WBP_Clue.HideArrowDrawer` _aswbp_clue)
  (`/Game/UI/Widgets/clue/WBP_Clue.HideArrowReturn` _aswbp_clue)
  (`/Game/UI/Widgets/clue/WBP_Clue.HideVillagerImage` _aswbp_clue))

(fn `Return`
  (bind _returnvalue (`/Game/Blueprints/BP_FL_shortcut.GetDrawer`))
  (if (`self.InDrawer`)
    (`self.Interraction` _returnvalue)
    (`self.SetControllerVariable` _returnvalue)
    (`self.K2_DestroyActor`)
    (`Controller.ResetIgnoreLookInput` (`/Game/Blueprints/BP_FL_shortcut.GetController`))
    (`GameplayStatics.SetViewportMouseCaptureMode` "CapturePermanently_IncludingInitialMouseDown")
    (elif (`self.InBoard`)
      (`self.DezoomBoard`)
      (set `/Game/FirstPerson/Blueprints/BP_FirstPersonPlayerController.ActorClick` (`/Game/Blueprints/BP_FL_shortcut.GetBoard`) (`/Game/Blueprints/BP_FL_shortcut.GetController`))
      (`self.DisableUI`)
      (bind _aswbp_arrow_return (cast `/Game/UI/Widgets/clue/WBP_ArrowReturn` (`WidgetComponent.GetWidget` (`/Game/Blueprints/Interractables/BP_I_Board.WidgetReturn` (`/Game/Blueprints/BP_FL_shortcut.GetBoard`)))))
      (`Widget.SetVisibility` _aswbp_arrow_return "Visible")
      (`Controller.ResetIgnoreLookInput` (`/Game/Blueprints/BP_FL_shortcut.GetController`))
      (`GameplayStatics.SetViewportMouseCaptureMode` "CapturePermanently_IncludingInitialMouseDown")
      (else
        (`self.ObjectDezoom`)
        (`self.VariableReturn`)
        (`self.DisableUI`)
        (`Controller.ResetIgnoreLookInput` (`/Game/Blueprints/BP_FL_shortcut.GetController`))
        (`GameplayStatics.SetViewportMouseCaptureMode` "CapturePermanently_IncludingInitialMouseDown")))))

(fn `TeleportToBoard`
  (bind (_returnvalue_location _returnvalue_rotation) (`KismetMathLibrary.BreakTransform` (`self.GetTransform`)))
  (bind _returnvalue (`SceneComponent.K2_GetComponentToWorld` (`/Game/Blueprints/Interractables/BP_I_Board.SpawnClue` (`/Game/Blueprints/BP_FL_shortcut.GetBoard`))))
  (`SceneComponent.K2_SetWorldTransform` (`self.DefaultSceneRoot`) (`KismetMathLibrary.MakeTransform` (.location _returnvalue) (`KismetMathLibrary.MakeRotator` (.roll (.rotation _returnvalue)) (.pitch (.rotation _returnvalue)) (+ (.yaw (.rotation _returnvalue)) 360.0))) false false)
  (set `self.OriginalLocation` _returnvalue_location)
  (set `self.OriginalRotation` _returnvalue_rotation)
  (`self.DisableUI`)
  (set `self.InBoard` true)
  (`PrimitiveComponent.SetCollisionProfileName` (`self.StaticMesh`) "BlockAllDynamic" true))

(fn `UserConstructionScript`
  (`parent.UserConstructionScript`))