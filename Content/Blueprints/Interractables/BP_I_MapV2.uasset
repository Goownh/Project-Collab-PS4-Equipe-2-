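; Interactable map Blueprint that shows a pawn mesh on a tiled map, with world-space widgets for returning and for confirming a move.
; MovePawn converts a tile's widget-space position and size into the tile's scaled center, swapping axes, and moves the pawn there.
; ShowValidation and CloseValidation swap UI collision between the confirmation and return widgets, with the confirmation hidden at start.
; SetUI and DisableUI toggle the return widget's visibility and collision.
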(event `self.ReceiveBeginPlay`
  (`parent.ReceiveBeginPlay`)
  (`self.CloseValidation`))

(event `MovePawn`
  (params (`Tile Relative Location Y` :type "Float (double-precision)") (`Tile Relative Size X` :type "Float (double-precision)") (`Tile Relative Location X` :type "Float (double-precision)") (`Tile Relative Size Y` :type "Float (double-precision)"))
  (`KismetSystemLibrary.MoveComponentTo` (`self.SM_Pawn`) (`KismetMathLibrary.MakeVector` (* (+ `Tile Relative Location Y` (/ `Tile Relative Size X` 2.0)) -0.04) (* (+ `Tile Relative Location X` (/ `Tile Relative Size Y` 2.0)) 0.045) 2.0)))

(fn `CloseValidation`
  (bind _widgetvalidationmove (`self.WidgetValidationMove`))
  (`SceneComponent.SetVisibility` _widgetvalidationmove false false)
  (`PrimitiveComponent.SetCollisionProfileName` _widgetvalidationmove "NoCollision" true)
  (`PrimitiveComponent.SetCollisionProfileName` (`self.WidgetReturn`) "UI" true))

(fn `DisableUI`
  (`SceneComponent.SetVisibility` (`self.WidgetReturn`) false false)
  (`PrimitiveComponent.SetCollisionProfileName` (`self.WidgetReturn`) "NoCollision" true))

(fn `SetUI`
  (`PrimitiveComponent.SetCollisionProfileName` (`self.WidgetReturn`) "UI" true)
  (`SceneComponent.SetVisibility` (`self.WidgetReturn`) true false))

(fn `ShowValidation`
  (bind _widgetvalidationmove (`self.WidgetValidationMove`))
  (`PrimitiveComponent.SetCollisionProfileName` (`self.WidgetReturn`) "NoCollision" true)
  (`SceneComponent.SetVisibility` _widgetvalidationmove true false)
  (`PrimitiveComponent.SetCollisionProfileName` _widgetvalidationmove "UI" true)
  (bind _aswbp_validation_move (cast `/Game/UI/Widgets/Map/WBP_ValidationMove` (`WidgetComponent.GetWidget` _widgetvalidationmove)))
  (`/Game/UI/Widgets/Map/WBP_ValidationMove.SetPlaceName` _aswbp_validation_move))

(fn `UserConstructionScript`
  (`parent.UserConstructionScript`))