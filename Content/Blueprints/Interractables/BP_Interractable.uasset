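; Base Blueprint for interactable objects, with overridable interaction and UI hooks left empty for children.
; Hovering the cursor applies an outline overlay to the mesh, unless the controller is already interacting.
; Objects can either fly by timeline to the character's Plane and back, or become the blended camera view target.
; Helper functions switch controller interaction state, input mode, cursor and look lock, and restore them on return.
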(event `self.ReceiveBeginPlay`
  (bind _staticmesh (`self.StaticMesh`))
  ; Set les variables des transform originaux du static mesh
  (set `self.OriginalLocation` (`SceneComponent.K2_GetComponentLocation` _staticmesh))
  (set `self.OriginalRotation` (`SceneComponent.K2_GetComponentRotation` _staticmesh))
  (set `self.originalScale` (`SceneComponent.K2_GetComponentScale` _staticmesh)))

(event `ObjectZoom`
  (bind (_returnvalue_location _returnvalue_rotation) (`KismetMathLibrary.BreakTransform` (`SceneComponent.K2_GetComponentToWorld` (`/Game/FirstPerson/Blueprints/BP_FirstPersonCharacter.Plane` (`/Game/Blueprints/BP_FL_shortcut.GetCharacter`)))))
  ; L'objet vient à nous (surtout pour les rapports)
  (`Controller.SetIgnoreLookInput` (`GameplayStatics.GetPlayerController` 0) true)
  (bind (_direction _newtrack_0) (`Timeline|Timeline` :!via `PlayFromStart`)
    (:`Update`
      (`SceneComponent.K2_SetWorldTransform` (`self.StaticMesh`) (`KismetMathLibrary.MakeTransform` (`KismetMathLibrary.VLerp` (`self.OriginalLocation`) _returnvalue_location _newtrack_0) (`KismetMathLibrary.RLerp` (`self.OriginalRotation`) _returnvalue_rotation _newtrack_0) (`self.originalScale`)) false false))))

(event `ObjectDezoom`
  (bind (_returnvalue_location _returnvalue_rotation) (`KismetMathLibrary.BreakTransform` (`SceneComponent.K2_GetComponentToWorld` (`/Game/FirstPerson/Blueprints/BP_FirstPersonCharacter.Plane` (`/Game/Blueprints/BP_FL_shortcut.GetCharacter`)))))
  ; Permet de remettre l'objet en place
  (`Controller.ResetIgnoreLookInput` (`GameplayStatics.GetPlayerController` 0))
  (bind (_direction _newtrack_0) (`Timeline|Timeline_0` :!via `PlayFromStart`)
    (:`Update`
      (`SceneComponent.K2_SetWorldTransform` (`self.StaticMesh`) (`KismetMathLibrary.MakeTransform` (`KismetMathLibrary.VLerp` _returnvalue_location (`self.OriginalLocation`) _newtrack_0) (`KismetMathLibrary.RLerp` _returnvalue_rotation (`self.OriginalRotation`) _newtrack_0) (`self.originalScale`)) false false))))

(event `Interraction`
  ; Fonction a overide par les enfants
)

(event `self.StaticMesh.OnBeginCursorOver`
  (params (TouchedComponent :type "PrimitiveComponent Object Reference"))
  (bind _staticmesh (`self.StaticMesh`))
  (if (not (`/Game/FirstPerson/Blueprints/BP_FirstPersonPlayerController.Interract` (`/Game/Blueprints/BP_FL_shortcut.GetController`)))
    (`MeshComponent.SetOverlayMaterial` _staticmesh "/Game/Materials/VFX/M_Outline.M_Outline")
    (`PrimitiveComponent.SetFirstPersonPrimitiveType` _staticmesh "WorldSpaceRepresentation")))

(event `self.StaticMesh.OnEndCursorOver`
  (params (TouchedComponent :type "PrimitiveComponent Object Reference"))
  (bind _staticmesh (`self.StaticMesh`))
  (`MeshComponent.SetOverlayMaterial` _staticmesh null)
  (`PrimitiveComponent.SetFirstPersonPrimitiveType` _staticmesh "None"))

(fn `CameraChange`
  (`self.CameraZoom`))

(fn `CameraDezoom`
  (`PlayerController.SetViewTargetWithBlend` (`/Game/Blueprints/BP_FL_shortcut.GetController`) (`/Game/Blueprints/BP_FL_shortcut.GetCharacter`) 0.5 "VTBlend_Linear" 0.0 false))

(fn `CameraZoom`
  (`PlayerController.SetViewTargetWithBlend` (`/Game/Blueprints/BP_FL_shortcut.GetController`) self 0.5 "VTBlend_Linear" 0.0 false))

(fn `DisableUI`)

(fn `Return`
  (`self.CameraDezoom`)
  (`self.DisableUI`)
  (`self.VariableReturn`))

(fn `SetControllerVariable`
  (bind _asbp_first_person_player_controller (`/Game/Blueprints/BP_FL_shortcut.GetController`))
  (bind _staticmesh (`self.StaticMesh`))
  (set `/Game/FirstPerson/Blueprints/BP_FirstPersonPlayerController.ActorClick` self _asbp_first_person_player_controller)
  (set `/Game/FirstPerson/Blueprints/BP_FirstPersonPlayerController.Interract` true _asbp_first_person_player_controller)
  (set `PlayerController.bShowMouseCursor` true _asbp_first_person_player_controller)
  (`Controller.SetIgnoreLookInput` (`/Game/Blueprints/BP_FL_shortcut.GetController`) true)
  (`WidgetBlueprintLibrary.SetInputMode_GameAndUIEx` (`/Game/Blueprints/BP_FL_shortcut.GetController`) null "DoNotLock" false)
  (`MeshComponent.SetOverlayMaterial` _staticmesh null)
  (`PrimitiveComponent.SetFirstPersonPrimitiveType` _staticmesh "None"))

(fn `SetUI`)

(fn `UserConstructionScript`)

(fn `VariableReturn`
  (bind _asbp_first_person_player_controller (`/Game/Blueprints/BP_FL_shortcut.GetController`))
  (set `/Game/FirstPerson/Blueprints/BP_FirstPersonPlayerController.Interract` false _asbp_first_person_player_controller)
  (set `PlayerController.bShowMouseCursor` false _asbp_first_person_player_controller)
  (set `/Game/FirstPerson/Blueprints/BP_FirstPersonPlayerController.ActorClick` null _asbp_first_person_player_controller)
  (`WidgetBlueprintLibrary.SetInputMode_GameOnly` _asbp_first_person_player_controller)
  (`Controller.ResetIgnoreLookInput` (`/Game/Blueprints/BP_FL_shortcut.GetController`))
  (`GameplayStatics.SetViewportMouseCaptureMode` "CapturePermanently_IncludingInitialMouseDown"))