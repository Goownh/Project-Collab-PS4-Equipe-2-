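; Interactable board with a clickable pin box and stamp, each opening its own widget (pin box or color picker) while the board is the controller's clicked actor.
; Interaction switches input to Game and UI; opening a tool hides the return arrow, switches to UI-only input and sets BusyOnObject.
; Hovering a tool while not busy adds an outline overlay and first-person rendering.
; Helper functions toggle widget visibility together with collision profiles, with all UI disabled on BeginPlay.
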(event `self.ReceiveBeginPlay`
  (`parent.ReceiveBeginPlay`)
  (`self.DisableUI`))

(event `self.Interraction`
  (`WidgetBlueprintLibrary.SetInputMode_GameAndUIEx` (`/Game/Blueprints/BP_FL_shortcut.GetController`) null "DoNotLock" false))

(event `self.PinBox.OnClicked`
  (params (TouchedComponent :type "PrimitiveComponent Object Reference") (ButtonPressed :type "Key Structure"))
  (bind _widgetpinbox (`self.WidgetPinBox`))
  ; Affiche l'ui pour la boite de punaise et cache l'ui de base du tableau
  (if (== (`GameplayStatics.GetObjectClass` (`/Game/FirstPerson/Blueprints/BP_FirstPersonPlayerController.ActorClick` (`/Game/Blueprints/BP_FL_shortcut.GetController`))) "BP_I_Board_C")
    (`self.HiddenReturn`)
    (bind _aswbp_pin_box (cast `/Game/UI/Widgets/Board/WBP_pinBox` (`WidgetComponent.GetWidget` _widgetpinbox)))
    (`Widget.SetVisibility` _aswbp_pin_box "Visible")
    (`PrimitiveComponent.SetCollisionProfileName` _widgetpinbox "UI" true)
    (`WidgetBlueprintLibrary.SetInputMode_UIOnlyEx` (`/Game/Blueprints/BP_FL_shortcut.GetController`) null)
    (set `self.BusyOnObject` true)))

(event `self.Stamp.OnClicked`
  (params (TouchedComponent :type "PrimitiveComponent Object Reference") (ButtonPressed :type "Key Structure"))
  (bind _widgetcolor (`self.WidgetColor`))
  ; Affiche l'ui pour le tampon et désactive l'ui de base du tableau
  (if (== (`GameplayStatics.GetObjectClass` (`/Game/FirstPerson/Blueprints/BP_FirstPersonPlayerController.ActorClick` (`/Game/Blueprints/BP_FL_shortcut.GetController`))) "BP_I_Board_C")
    (`self.HiddenReturn`)
    (bind _aswbp_color_picker (cast `/Game/UI/Widgets/Board/WBP_ColorPicker` (`WidgetComponent.GetWidget` _widgetcolor)))
    (`Widget.SetVisibility` _aswbp_color_picker "Visible")
    (`PrimitiveComponent.SetCollisionProfileName` _widgetcolor "UI" true)
    (`WidgetBlueprintLibrary.SetInputMode_UIOnlyEx` (`/Game/Blueprints/BP_FL_shortcut.GetController`) null)
    (set `self.BusyOnObject` true)))

(event `self.PinBox.OnBeginCursorOver`
  (params (TouchedComponent :type "PrimitiveComponent Object Reference"))
  (bind _pinbox (`self.PinBox`))
  (if (and (== (`GameplayStatics.GetObjectClass` (`/Game/FirstPerson/Blueprints/BP_FirstPersonPlayerController.ActorClick` (`/Game/Blueprints/BP_FL_shortcut.GetController`))) "BP_I_Board_C") (== (`self.BusyOnObject`) false))
    (`MeshComponent.SetOverlayMaterial` _pinbox "/Game/Materials/VFX/M_Outline.M_Outline")
    (`PrimitiveComponent.SetFirstPersonPrimitiveType` _pinbox "FirstPerson")))

(event `self.PinBox.OnEndCursorOver`
  (params (TouchedComponent :type "PrimitiveComponent Object Reference"))
  (bind _pinbox (`self.PinBox`))
  (`MeshComponent.SetOverlayMaterial` _pinbox null)
  (`PrimitiveComponent.SetFirstPersonPrimitiveType` _pinbox "None"))

(event `self.Stamp.OnBeginCursorOver`
  (params (TouchedComponent :type "PrimitiveComponent Object Reference"))
  (bind _stamp (`self.Stamp`))
  (if (and (== (`GameplayStatics.GetObjectClass` (`/Game/FirstPerson/Blueprints/BP_FirstPersonPlayerController.ActorClick` (`/Game/Blueprints/BP_FL_shortcut.GetController`))) "BP_I_Board_C") (== (`self.BusyOnObject`) false))
    (`MeshComponent.SetOverlayMaterial` _stamp "/Game/Materials/VFX/M_Outline.M_Outline")
    (`PrimitiveComponent.SetFirstPersonPrimitiveType` _stamp "FirstPerson")))

(event `self.Stamp.OnEndCursorOver`
  (params (TouchedComponent :type "PrimitiveComponent Object Reference"))
  (bind _stamp (`self.Stamp`))
  (`MeshComponent.SetOverlayMaterial` _stamp null)
  (`PrimitiveComponent.SetFirstPersonPrimitiveType` _stamp "None"))

(fn `DisableUI`
  (bind _widgetreturn (`self.WidgetReturn`))
  (bind _widgetcolor (`self.WidgetColor`))
  (bind _widgetpinbox (`self.WidgetPinBox`))
  (bind _aswbp_arrow_return (cast `/Game/UI/Widgets/clue/WBP_ArrowReturn` (`WidgetComponent.GetWidget` _widgetreturn)))
  (set `Widget.Visibility` "Hidden" (`/Game/UI/Widgets/clue/WBP_ArrowReturn.Button_61` _aswbp_arrow_return))
  (`PrimitiveComponent.SetCollisionProfileName` _widgetreturn "NoCollision" true)
  (bind _aswbp_color_picker (cast `/Game/UI/Widgets/Board/WBP_ColorPicker` (`WidgetComponent.GetWidget` _widgetcolor)))
  (`Widget.SetVisibility` _aswbp_color_picker "Hidden")
  (`PrimitiveComponent.SetCollisionProfileName` _widgetcolor "NoCollision" true)
  (bind _aswbp_pin_box (cast `/Game/UI/Widgets/Board/WBP_pinBox` (`WidgetComponent.GetWidget` _widgetpinbox)))
  (`Widget.SetVisibility` _aswbp_pin_box "Hidden")
  (`PrimitiveComponent.SetCollisionProfileName` _widgetpinbox "NoCollision" true))

(fn `HiddenReturn`
  (bind _widgetreturn (`self.WidgetReturn`))
  (bind _aswbp_arrow_return (cast `/Game/UI/Widgets/clue/WBP_ArrowReturn` (`WidgetComponent.GetWidget` _widgetreturn)))
  (`Widget.SetVisibility` (`/Game/UI/Widgets/clue/WBP_ArrowReturn.Button_61` _aswbp_arrow_return) "Hidden")
  (`PrimitiveComponent.SetCollisionProfileName` _widgetreturn "NoCollision" true))

(fn `SetUI`
  (bind _widgetreturn (`self.WidgetReturn`))
  (bind _aswbp_arrow_return (cast `/Game/UI/Widgets/clue/WBP_ArrowReturn` (`WidgetComponent.GetWidget` _widgetreturn)))
  (set `Widget.Visibility` "Visible" (`/Game/UI/Widgets/clue/WBP_ArrowReturn.Button_61` _aswbp_arrow_return))
  (`PrimitiveComponent.SetCollisionProfileName` _widgetreturn "UI" true))

(fn `UserConstructionScript`
  (`parent.UserConstructionScript`))