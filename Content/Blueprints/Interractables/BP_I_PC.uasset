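; Interactable PC with in-world widget screens: a menu, a WhatsApp chat with clue pages, a Paint app and empty Word stubs.
; The first interaction turns on the menu and return button.
; Open/close functions toggle visibility and UI collision, tracking CurrentWidget so SetUI can re-enable input after DisableUI.
; Paint adds a brush widget to the viewport and opens BPCanvas; PrintClue calls the printer found at BeginPlay.
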(event `self.ReceiveBeginPlay`
  (`parent.ReceiveBeginPlay`)
  (`self.DisableUIStart`)
  ; Connect PC to Printer
  (bind _outactors (`GameplayStatics.GetAllActorsOfClass` "/Game/Blueprints/Interractables/BP_I_Printer.BP_I_Printer_C"))
  (for _array_element _outactors
    (set `self.Printer` _array_element)))

(event `self.Interraction`
  (if (not (`self.On`))
    (`self.SetUIStart`)
    (set `self.On` true)))

(event `self.ReceiveTick`
  (params (DeltaSeconds :type "Float (single-precision)")))

(fn `CloseCluePage`
  (bind _whatsappcluescreen (`self.WhatsAppClueScreen`))
  (bind _whatsappscreen (`self.WhatsAppScreen`))
  (`SceneComponent.SetVisibility` _whatsappcluescreen false true)
  (`PrimitiveComponent.SetCollisionProfileName` _whatsappcluescreen "NoCollision" true)
  (`PrimitiveComponent.SetCollisionProfileName` _whatsappscreen "UI" true)
  (set `self.CurrentWidget` _whatsappscreen))

(fn `CloseMenu`
  (bind _menu (`self.Menu`))
  (`SceneComponent.SetVisibility` _menu false true)
  (`PrimitiveComponent.SetCollisionProfileName` _menu "NoCollision" true))

(fn `ClosePaint`
  (bind _paintscreen (`self.PaintScreen`))
  (`Widget.RemoveFromParent` (`self.PaintBrush`))
  (`/Game/Blueprints/BP_Canvas.CloseCanvas` (`self.BP Canvas`))
  (`SceneComponent.SetVisibility` _paintscreen false true)
  (`PrimitiveComponent.SetCollisionProfileName` _paintscreen "NoCollision" true)
  (`self.OpenMenu`))

(fn `CloseWhatsApp`
  (bind _whatsappscreen (`self.WhatsAppScreen`))
  (`SceneComponent.SetVisibility` _whatsappscreen false true)
  (`PrimitiveComponent.SetCollisionProfileName` _whatsappscreen "NoCollision" true)
  (`self.OpenMenu`))

(fn `CloseWord`)

(fn `DisableUI`
  (`PrimitiveComponent.SetCollisionProfileName` (`self.Menu`) "NoCollision" true)
  (`PrimitiveComponent.SetCollisionProfileName` (`self.WhatsAppScreen`) "NoCollision" true)
  (`PrimitiveComponent.SetCollisionProfileName` (`self.WhatsAppClueScreen`) "NoCollision" true)
  (`PrimitiveComponent.SetCollisionProfileName` (`self.PaintScreen`) "NoCollision" true)
  (`PrimitiveComponent.SetCollisionProfileName` (`/Game/Blueprints/BP_Canvas.Plane` (`self.BP Canvas`)) "NoCollision" true))

(fn `DisableUIStart`
  (bind _menu (`self.Menu`))
  (bind _whatsappcluescreen (`self.WhatsAppClueScreen`))
  (bind _whatsappscreen (`self.WhatsAppScreen`))
  (bind _returnbutton (`self.ReturnButton`))
  (bind _paintscreen (`self.PaintScreen`))
  ; Disable Menu
  (`PrimitiveComponent.SetCollisionProfileName` _menu "NoCollision" true)
  (`SceneComponent.SetVisibility` _menu false true)
  ; Disable WhatsAppScreen
  (`PrimitiveComponent.SetCollisionProfileName` _whatsappscreen "NoCollision" true)
  (`SceneComponent.SetVisibility` _whatsappscreen false true)
  ; Disable WhatsAppClueScreen
  (`PrimitiveComponent.SetCollisionProfileName` _whatsappcluescreen "NoCollision" true)
  (`SceneComponent.SetVisibility` _whatsappcluescreen false true)
  ; Disable PaintScreen
  (`PrimitiveComponent.SetCollisionProfileName` _paintscreen "NoCollision" true)
  (`SceneComponent.SetVisibility` _paintscreen false true)
  (`/Game/Blueprints/BP_Canvas.CloseCanvas` (`self.BP Canvas`))
  ; Hide ReturnButton
  (bind _aswbp_arrow_return (cast `/Game/UI/Widgets/clue/WBP_ArrowReturn` (`WidgetComponent.GetWidget` _returnbutton)))
  (set `Widget.Visibility` "Hidden" (`/Game/UI/Widgets/clue/WBP_ArrowReturn.Button_61` _aswbp_arrow_return))
  (`PrimitiveComponent.SetCollisionProfileName` _returnbutton "NoCollision" true))

(fn `NewCluePage`
  (params (Clue :type String))
  (bind _whatsappcluescreen (`self.WhatsAppClueScreen`))
  (`SceneComponent.SetVisibility` _whatsappcluescreen true true)
  (`PrimitiveComponent.SetCollisionProfileName` _whatsappcluescreen "UI" true)
  (bind _aswbp_pcwhats_app_clue (cast `/Game/UI/Widgets/PC/WhatsApp/WBP_PCWhatsAppClue` (`WidgetComponent.GetWidget` _whatsappcluescreen)))
  (`/Game/UI/Widgets/PC/WhatsApp/WBP_PCWhatsAppClue.SetClue` _aswbp_pcwhats_app_clue Clue)
  (`PrimitiveComponent.SetCollisionProfileName` (`self.WhatsAppScreen`) "NoCollision" true)
  (set `self.CurrentWidget` (`self.WhatsAppClueScreen`)))

(fn `OpenMenu`
  (bind _menu (`self.Menu`))
  (`SceneComponent.SetVisibility` _menu true true)
  (`PrimitiveComponent.SetCollisionProfileName` _menu "UI" true)
  (set `self.CurrentWidget` _menu))

(fn `OpenPaint`
  (bind _paintscreen (`self.PaintScreen`))
  (bind _returnvalue (`|GenericCreateObject` (`/Game/Blueprints/BP_FL_shortcut.GetCharacter`) "/Game/UI/Widgets/PC/Paint/WBP_PCPaintBrush.WBP_PCPaintBrush_C"))
  (bind _output_get (set `self.PaintBrush` _returnvalue))
  (`UserWidget.AddToViewport` _output_get 0)
  (`self.CloseMenu`)
  (`/Game/Blueprints/BP_Canvas.OpenCanvas` (`self.BP Canvas`))
  (`SceneComponent.SetVisibility` _paintscreen true true)
  (`PrimitiveComponent.SetCollisionProfileName` _paintscreen "UI" true)
  (set `self.CurrentWidget` _paintscreen))

(fn `OpenWhatsApp`
  (bind _whatsappscreen (`self.WhatsAppScreen`))
  (`self.CloseMenu`)
  (`SceneComponent.SetVisibility` _whatsappscreen true true)
  (`PrimitiveComponent.SetCollisionProfileName` _whatsappscreen "UI" true)
  (set `self.CurrentWidget` _whatsappscreen))

(fn `OpenWord`)

(fn `PrintClue`
  (`/Game/Blueprints/Interractables/BP_I_Printer.PrintClue` (`self.Printer`) ""))

(fn `SetUI`
  (bind _returnbutton (`self.ReturnButton`))
  (bind _currentwidget (`self.CurrentWidget`))
  (if (!= _currentwidget null)
    (if (not (!= (`self.PaintScreen`) _currentwidget))
      (`PrimitiveComponent.SetCollisionProfileName` (`/Game/Blueprints/BP_Canvas.Plane` (`self.BP Canvas`)) "UI" true))
    (`PrimitiveComponent.SetCollisionProfileName` _currentwidget "UI" true)
    (`PrimitiveComponent.SetCollisionProfileName` _returnbutton "UI" true)
    (bind _aswbp_arrow_return (cast `/Game/UI/Widgets/clue/WBP_ArrowReturn` (`WidgetComponent.GetWidget` _returnbutton)))
    (set `Widget.Visibility` "Visible" (`/Game/UI/Widgets/clue/WBP_ArrowReturn.Button_61` _aswbp_arrow_return))))

(fn `SetUIStart`
  (bind _returnbutton (`self.ReturnButton`))
  (bind _menu (`self.Menu`))
  ; Start Menu
  (`PrimitiveComponent.SetCollisionProfileName` _menu "UI" true)
  (`SceneComponent.SetVisibility` _menu true true)
  (`PrimitiveComponent.SetCollisionProfileName` _returnbutton "UI" true)
  (bind _aswbp_arrow_return (cast `/Game/UI/Widgets/clue/WBP_ArrowReturn` (`WidgetComponent.GetWidget` _returnbutton)))
  (set `Widget.Visibility` "Visible" (`/Game/UI/Widgets/clue/WBP_ArrowReturn.Button_61` _aswbp_arrow_return))
  (set `self.CurrentWidget` (`self.Menu`)))

(fn `UserConstructionScript`)