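; Interactable letter that opens the investigation tutorial, showing a placeholder voice line on day 0 that prompts the player to read it.
; Each interaction unlocks the map for the tutorial and spawns a BP_I_Clue at the character's Plane, fed the next NameLetter entry.
; Once the list is empty, it prints a line directing the field agent to the town hall, clears every door's Letter reference and destroys itself.
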(event `self.ReceiveBeginPlay`
  (`parent.ReceiveBeginPlay`)
  ; Set usable
  (set `self.UsableForTuto` true)
  (if (== (`/Game/Blueprints/Interractables/BP_I_Door.CurrentDay` (`/Game/Blueprints/BP_FL_shortcut.GetDoor`)) 0)
    (`KismetSystemLibrary.PrintText` "VA \"Nouveau jour, nouvelle enquete. Je devrait commencer par lire la lettre que l'on m'a envoyé.\"" true true (struct :`R` 1.0 :`A` 1.0) 10.0)))

(event `self.Interraction`
  (bind (_returnvalue_location _returnvalue_rotation) (`KismetMathLibrary.BreakTransform` (`SceneComponent.K2_GetComponentToWorld` (`/Game/FirstPerson/Blueprints/BP_FirstPersonCharacter.Plane` (`/Game/Blueprints/BP_FL_shortcut.GetCharacter`)))))
  (bind _returnvalue (`GameplayStatics.GetActorOfClass` "/Game/Blueprints/Interractables/BP_I_Map.BP_I_Map_C"))
  (set `/Game/Blueprints/Interractables/BP_I_Map.UsableForTuto` true _returnvalue)
  (if (> (`KismetArrayLibrary.Array_Length` (`self.NameLetter`)) 0)
    (bind _returnvalue_2 (`|SpawnActorFromClass` "/Game/Blueprints/Interractables/BP_I_Clue.BP_I_Clue_C" (`KismetMathLibrary.MakeTransform` _returnvalue_location _returnvalue_rotation) "AlwaysSpawn" "OverrideRootScale" null null))
    (set `/Game/Blueprints/Interractables/BP_I_Clue.Id_rapport` (`|GetArrayItem` (`self.NameLetter`)) _returnvalue_2)
    (`/Game/Blueprints/Interractables/BP_I_Clue.Letter` _returnvalue_2)
    (`KismetArrayLibrary.Array_Remove` (`self.NameLetter`))
    (else
      (`self.Destroy`)
      (`KismetSystemLibrary.PrintText` "VA \"Huuummmm je voit. Déplaçons mon agent de terrrain a la mairie afin d'en apprendre plus\"" true true (struct :`R` 1.0 :`A` 1.0) 10.0))))

(fn `CameraChange`)

(fn `Destroy`
  (`self.Return`)
  (bind _outactors (`GameplayStatics.GetAllActorsOfClass` "/Game/Blueprints/Interractables/BP_I_Door.BP_I_Door_C"))
  (for _array_element _outactors
    (set `/Game/Blueprints/Interractables/BP_I_Door.Letter` null _array_element))
  (`self.K2_DestroyActor`))

(fn `UserConstructionScript`
  (`parent.UserConstructionScript`))