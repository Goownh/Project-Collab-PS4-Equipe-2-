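; Interactable door that advances the game's day cycle and, on the final day, resolves the culprit vote.
; Interaction opens a day confirmation, or a vote confirmation once a villager is chosen on the last day.
; WayDay swings the door by Timeline, increments the day, resets moves and map tiles, and spawns that day's clue letter from DT_ListClue.
; VerificationVote checks villager pictures and the chosen culprit to show a win or lose pay stub.
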(event `self.ReceiveBeginPlay`
  (`parent.ReceiveBeginPlay`)
  (bind _outactors (`GameplayStatics.GetAllActorsOfClass` "/Game/Blueprints/BP_SpawnLetter.BP_SpawnLetter_C"))
  (for _array_element _outactors
    (set `self.SpawnLetter` _array_element))
  (`self.MakeLetter`)
  ; Afficher et désafficher le jour actuel
  (bind _returnvalue (`|CreateWidget` "/Game/UI/Widgets/Day/WBP_NewDay.WBP_NewDay_C"))
  (bind _output_get (set `self.UIDay` _returnvalue))
  (`UserWidget.AddToViewport` _output_get 0)
  (`/Game/UI/Widgets/Day/WBP_NewDay.SetCurrentDay` _returnvalue self)
  (`KismetSystemLibrary.Delay` 2.0)
  (`Widget.RemoveFromParent` (`self.UIDay`)))

(event `self.Interraction`
  (if (< (`self.CurrentDay`) (`self.DayMax`))
    (if (`/Game/Blueprints/BP_FL_shortcut.GetIsTuto`)
      (bind _outactors (`GameplayStatics.GetAllActorsOfClass` "/Game/Blueprints/Interractables/BP_Interractable.BP_Interractable_C"))
      (for _array_element _outactors
        (set `/Game/Blueprints/Interractables/BP_Interractable.UsableForTuto` true _array_element)))
    (bind _returnvalue (`|CreateWidget` "/Game/UI/Widgets/Door/WBP_DayConfirmation.WBP_DayConfirmation_C"))
    (bind _output_get (set `self.UIDayConfirmation` _returnvalue))
    (`UserWidget.AddToViewport` _output_get 0)
    (elif (`KismetStringLibrary.EqualEqual_StrStr` (`/Game/FirstPerson/Blueprints/BP_FirstPersonCharacter.ChosenVillager` (`/Game/Blueprints/BP_FL_shortcut.GetCharacter`)))
      (`self.Return`)
      (else
        (bind _returnvalue_2 (`|CreateWidget` "/Game/UI/Widgets/Door/WBP_VoteConfirmation.WBP_VoteConfirmation_C"))
        (bind _output_get_2 (set `self.UIVoteConfirmation` _returnvalue_2))
        (`UserWidget.AddToViewport` _output_get_2 0)))))

(event `WayDay`
  (bind _asbp_first_person_character (`/Game/Blueprints/BP_FL_shortcut.GetCharacter`))
  (bind _asbp_first_person_character_2 (`/Game/Blueprints/BP_FL_shortcut.GetCharacter`))
  (bind _staticmesh (`self.StaticMesh`))
  (bind _letter (`self.Letter`))
  (bind (_returnvalue_roll _returnvalue_pitch _returnvalue_yaw) (`KismetMathLibrary.BreakRotator` (`SceneComponent.K2_GetComponentRotation` _staticmesh)))
  (`/Game/FirstPerson/Blueprints/BP_FirstPersonCharacter.NewDay` (`/Game/Blueprints/BP_FL_shortcut.GetCharacter`))
  (`self.RemoveUIDayConfirmation`)
  (`Controller.SetIgnoreLookInput` (`/Game/Blueprints/BP_FL_shortcut.GetController`) true)
  ; Rotation porte
  (`Timeline|Timeline_1` :!via `PlayFromStart`
    (:`Update`
      (`SceneComponent.K2_SetWorldRotation` _staticmesh (`KismetMathLibrary.MakeRotator` _returnvalue_roll _returnvalue_pitch (+ _returnvalue_yaw 1.0)) false false))
    (:`Finished`
      (`KismetSystemLibrary.Delay` 0.5)
      ; Remise à l'état d'origine de la porte
      (`SceneComponent.K2_SetWorldRotation` (`self.StaticMesh`) (`self.OriginalRotation`) false false)
      (set `self.CurrentDay` (+ (`self.CurrentDay`) 1))
      ; Ouverture des yeux
      (set `/Game/FirstPerson/Blueprints/BP_FirstPersonCharacter.StartNewDay` false _asbp_first_person_character_2)
      (`/Game/FirstPerson/Blueprints/BP_FirstPersonCharacter.NewDay` _asbp_first_person_character_2)
      (set `/Game/FirstPerson/Blueprints/BP_FirstPersonCharacter.StartNewDay` true _asbp_first_person_character_2)
      (switch `int` (`self.CurrentDay`)
        (:`1`
          (set `/Game/FirstPerson/Blueprints/BP_FirstPersonCharacter.Moves` 5 _asbp_first_person_character))
        (:`2`
          (set `/Game/FirstPerson/Blueprints/BP_FirstPersonCharacter.Moves` 4 _asbp_first_person_character))
        (:`3`
          (set `/Game/FirstPerson/Blueprints/BP_FirstPersonCharacter.Moves` 3 _asbp_first_person_character :!label _label))
        (:`4`
          (goto _label))
        (:`5`
          (goto _label)))
      (bind _foundwidgets (`WidgetBlueprintLibrary.GetAllWidgetsOfClass` "/Game/UI/Widgets/Map/WBP_Map.WBP_Map_C" false))
      (for _array_element _foundwidgets
        (`/Game/UI/Widgets/Map/WBP_Map.SetMovesUI` _array_element))
      (bind _foundwidgets_2 (`WidgetBlueprintLibrary.GetAllWidgetsOfClass` "/Game/UI/Widgets/Map/WBP_Tile.WBP_Tile_C" false))
      (for _array_element_2 _foundwidgets_2
        (set `/Game/UI/Widgets/Map/WBP_Tile.ClickedToday` false _array_element_2))
      (if (not (== _letter null))
        (`/Game/Blueprints/Interractables/BP_I_letter.Destroy` _letter))
      (`self.MakeLetter`)
      (`Widget.RemoveFromParent` (`self.UIDay`))
      (bind _returnvalue (`|CreateWidget` "/Game/UI/Widgets/Day/WBP_NewDay.WBP_NewDay_C"))
      (bind _output_get (set `self.UIDay` _returnvalue))
      (`UserWidget.AddToViewport` _output_get 0)
      (`/Game/UI/Widgets/Day/WBP_NewDay.SetCurrentDay` _returnvalue self)
      (`KismetSystemLibrary.Delay` 2.0)
      (`Widget.RemoveFromParent` (`self.UIDay`))
      (`Controller.ResetIgnoreLookInput` (`/Game/Blueprints/BP_FL_shortcut.GetController`)))))

(fn `CameraZoom`)

(fn `MakeLetter`
  (bind _returnvalue (`|SpawnActorFromClass` "/Game/Blueprints/Interractables/BP_I_letter.BP_I_letter_C" (`self.GetTransform` (`self.SpawnLetter`)) "Undefined" "MultiplyWithRoot" null null))
  (bind _returnvalue_2 (`|GetDataTableRow` "/Game/Blueprints/Structures/DT_ListClue.DT_ListClue" (`KismetStringLibrary.Conv_StringToName` (`KismetStringLibrary.Conv_IntToString` (`self.CurrentDay`))))
    (:`then`
      (set `/Game/Blueprints/Interractables/BP_I_letter.NameLetter` (`.ListClue_4_CD8A7DF04823B440A0D2258994838DD7` (break `/Game/Blueprints/Structures/F_ListClue` _returnvalue_2)) _returnvalue)
      (set `self.Letter` _returnvalue))))

(fn `RemoveUIDayConfirmation`
  (`Widget.RemoveFromParent` (`self.UIDayConfirmation`))
  (set `self.UIDayConfirmation` null)
  (`self.Return`))

(fn `RemoveUIVoteConfirmation`
  (`Widget.RemoveFromParent` (`self.UIVoteConfirmation`))
  (set `self.UIVoteConfirmation` null)
  (`self.Return`))

(fn `UserConstructionScript`
  (`parent.UserConstructionScript`))

(fn `VerificationVote`
  (bind _asbp_first_person_character (`/Game/Blueprints/BP_FL_shortcut.GetCharacter`))
  (`self.RemoveUIVoteConfirmation`)
  ; Check si on peut avoir le score de fin
  (bind _outactors (`GameplayStatics.GetAllActorsOfClass` "/Game/Blueprints/Interractables/BP_I_VillagerPicture.BP_I_VillagerPicture_C"))
  (for _array_element _outactors
    (set `self.Win` (or (`self.Win`) (and (== (`/Game/Blueprints/Interractables/BP_I_VillagerPicture.Voted` _array_element) true) (== (`self.CurrentDay`) (`self.DayMax`)) (`KismetStringLibrary.EqualEqual_StrStr` (`/Game/FirstPerson/Blueprints/BP_FirstPersonCharacter.ChosenVillager` _asbp_first_person_character) (`/Game/FirstPerson/Blueprints/BP_FirstPersonCharacter.Culprit` _asbp_first_person_character))))))
  (if (`self.Win`)
    ;; Affichage de Gagné
    (bind _returnvalue (`|CreateWidget` "/Game/UI/Widgets/Score/WBP_PayStub.WBP_PayStub_C"))
    (`UserWidget.AddToPlayerScreen` _returnvalue 0)
    (else
      ;; Affichage de Perdu
      (bind _returnvalue_2 (`|CreateWidget` "/Game/UI/Widgets/Score/WBP_PayStubLose.WBP_PayStubLose_C"))
      (`UserWidget.AddToPlayerScreen` _returnvalue_2 0)))
  (`Controller.SetIgnoreLookInput` (`/Game/Blueprints/BP_FL_shortcut.GetController`) true))