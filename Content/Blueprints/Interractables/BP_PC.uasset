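; BP_PC is an interactable in-world computer that shows a WhatsApp screen and a separate clue page as widget components.
; On BeginPlay it gives both widgets a reference to itself, disables their collision and hides the clue screen; interaction makes the main screen clickable.
; NewCluePage and CloseCluePage switch collision profiles between UI and NoCollision so only one screen takes input.
; SetUI shows a return arrow on the ButtonReturn widget.
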(event `self.ReceiveBeginPlay`
  (bind _whatsappcluescreen (`self.WhatsAppClueScreen`))
  (bind _whatsappscreen (`self.WhatsAppScreen`))
  (`parent.ReceiveBeginPlay`)
  (`PrimitiveComponent.SetCollisionProfileName` _whatsappscreen "NoCollision" true)
  (bind _aswbp_pcwhats_app (cast `/Game/UI/Widgets/PC/WBP_PCWhatsApp` (`WidgetComponent.GetWidget` _whatsappscreen)))
  (set `/Game/UI/Widgets/PC/WBP_PCWhatsApp.Pc` self _aswbp_pcwhats_app)
  (`PrimitiveComponent.SetCollisionProfileName` _whatsappcluescreen "NoCollision" true)
  (`SceneComponent.SetVisibility` _whatsappcluescreen false true)
  (bind _aswbp_pcwhats_app_clue (cast `/Game/UI/Widgets/PC/WBP_PCWhatsAppClue` (`WidgetComponent.GetWidget` _whatsappcluescreen)))
  (set `/Game/UI/Widgets/PC/WBP_PCWhatsAppClue.Pc` self _aswbp_pcwhats_app_clue))

(event `self.Interraction`
  (`PrimitiveComponent.SetCollisionProfileName` (`self.WhatsAppScreen`) "UI" true))

(fn `CloseCluePage`
  (bind _whatsappcluescreen (`self.WhatsAppClueScreen`))
  (`SceneComponent.SetVisibility` _whatsappcluescreen false true)
  (`PrimitiveComponent.SetCollisionProfileName` _whatsappcluescreen "NoCollision" true)
  (`PrimitiveComponent.SetCollisionProfileName` (`self.WhatsAppScreen`) "UI" true))

(fn `DisableUI`)

(fn `NewCluePage`
  (params (Clue :type String))
  (bind _whatsappcluescreen (`self.WhatsAppClueScreen`))
  (`SceneComponent.SetVisibility` _whatsappcluescreen true true)
  (`PrimitiveComponent.SetCollisionProfileName` _whatsappcluescreen "UI" true)
  (bind _aswbp_pcwhats_app_clue (cast `/Game/UI/Widgets/PC/WBP_PCWhatsAppClue` (`WidgetComponent.GetWidget` _whatsappcluescreen)))
  (`/Game/UI/Widgets/PC/WBP_PCWhatsAppClue.SetClue` _aswbp_pcwhats_app_clue Clue)
  (`PrimitiveComponent.SetCollisionProfileName` (`self.WhatsAppScreen`) "NoCollision" true))

(fn `SetUI`
  (bind _aswbp_clue (cast `/Game/UI/Widgets/clue/WBP_Clue` (`WidgetComponent.GetWidget` (`self.ButtonReturn`))))
  (`/Game/UI/Widgets/clue/WBP_Clue.ShowArrowReturn` _aswbp_clue))

(fn `UserConstructionScript`)