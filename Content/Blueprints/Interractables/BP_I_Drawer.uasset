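; Interactable drawer that slides open and shows the clues it holds in a UI widget.
; Interraction plays an open sound, adds a WBP_drawer widget filled from ListClue, and runs a timeline that lerps the mesh from OriginalLocation to TargetPoint.
; Return calls the parent, removes the widget, reverses the timeline and plays a close sound.
; CameraChange is left empty.
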(event `self.ReceiveBeginPlay`
  (`parent.ReceiveBeginPlay`))

(event `self.Interraction`
  (`GameplayStatics.PlaySound2D` "/Game/Sounds/Drawer/SW_DrawerOpen.SW_DrawerOpen" 1.0 1.0 0.0 null null)
  (bind _returnvalue (`|CreateWidget` "/Game/UI/Widgets/drawer/WBP_drawer.WBP_drawer_C"))
  (bind _output_get (set `self.UIClue` _returnvalue))
  (`UserWidget.AddToViewport` _output_get 0)
  (`/Game/UI/Widgets/drawer/WBP_drawer.SetClue` _output_get (`self.ListClue`))
  (bind (_direction _newtrack_0) (`Timeline|Timeline_1` :!via `PlayFromStart` :!label _label)
    (:`Update`
      (`SceneComponent.K2_SetWorldLocation` (`self.StaticMesh`) (`KismetMathLibrary.VLerp` (`self.OriginalLocation`) (`SceneComponent.K2_GetComponentLocation` (`self.TargetPoint`)) _newtrack_0) false false))))

(event `AnimationClose`
  (goto _label :!via `ReverseFromEnd`))

(fn `CameraChange`)

(fn `Return`
  (`parent.Return`)
  (`Widget.RemoveFromParent` (`self.UIClue`))
  (`self.AnimationClose`)
  (`GameplayStatics.PlaySound2D` "/Game/Sounds/Drawer/SW_DrawerClose.SW_DrawerClose" 1.0 1.0 0.0 null null))

(fn `UserConstructionScript`
  (`parent.UserConstructionScript`))